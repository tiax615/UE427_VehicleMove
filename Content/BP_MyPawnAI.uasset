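; AI-driven vehicle pawn that drives itself along a navmesh path to a requested location.
; AIVehicleMoveTo finds a synchronous navigation path, stores its points, enables Tick and releases the handbrake.
; Tick steers from the unnormalized yaw difference to the current point, scales throttle by distance and advances when close.
; It draws debug points while driving and applies brake and handbrake once the path ends.
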(event EventBeginPlay)

(event Collision|EventActorBeginOverlap
  (params (OtherActor :type Actor%20Object%20Reference)))

(event EventTick
  (params (DeltaSeconds :type Float%20%28single-precision%29))
  (bind _returnvalue (Transformation|GetActorLocation))
  (bind _locationindex (Variables|Default|GetLocationIndex))
  (bind _locationarr (Variables|Default|GetLocationArr))
  (bind _vehiclemovement (Variables|Default|GetVehicleMovement))
  (bind _output (Utilities|Array|Get(acopy) _locationarr _locationindex))
  (bind _returnvalue_2 (Math|Vector|Distance(Vector) _output _returnvalue))
  (if (< (Variables|Default|GetLocationIndex) (Utilities|Array|Length (Variables|Default|GetLocationArr)))
    ;[1 1 1] Set Steering
    (Class|WheeledVehicleMovementComponent|SetSteeringInput (Variables|Default|GetVehicleMovement) (Math|Float|MapRangeClamped (- (.Yaw (Math|Rotator|BreakRotator (Math|Rotator|FindLookatRotation (Transformation|GetActorLocation) (Utilities|Array|Get(acopy) (Variables|Default|GetLocationArr) (Variables|Default|GetLocationIndex))))) (.Yaw (Math|Rotator|BreakRotator (Transformation|GetActorRotation)))) -9e+01 9e+01 -1.0 1.0))
    ;[1 1 1] Set Throttle
    (if (< _returnvalue_2 3e+02)
      (Math|Integer|IncrementInt (Variables|Default|GetLocationIndex))
      (else
        (Class|WheeledVehicleMovementComponent|SetThrottleInput (Variables|Default|GetVehicleMovement) (Math|Float|MapRangeClamped _returnvalue_2 0.0 1e+03 0.0 0.8))
        ;[1 1 1] Draw Debug Point
        (for _array_element (Variables|Default|GetLocationArr)
          (Rendering|Debug|DrawDebugPoint _array_element 1e+01 "(R=1.000000,G=0.000000,B=0.424941,A=1.000000)" 0.0))))
    (else
      ;[1 1 1] Stop
      (Class|WheeledVehicleMovementComponent|SetThrottleInput _vehiclemovement 0.0)
      (Class|WheeledVehicleMovementComponent|SetHandbrakeInput _vehiclemovement true)
      (Class|WheeledVehicleMovementComponent|SetBrakeInput _vehiclemovement 1.0))))

(fn ConstructionScript)

(fn AIVehicleMoveto
  (params (Location :type Vector))
  (bind _returnvalue (Class|NavigationSystemV1|FindPathtoLocationSynchronously (Class|NavigationSystemV1|GetNavigationSystem) (Transformation|GetActorLocation) Location self 0))
  (Utilities|IsValid _returnvalue
    (:Is%20Valid
      (Variables|Default|SetLocationArr (Variables|/Script/NavigationSystem.NavigationPath|GetPathPoints _returnvalue))
      (Actor|Tick|SetActorTickEnabled true)
      (Class|WheeledVehicleMovementComponent|SetHandbrakeInput (Variables|Default|GetVehicleMovement) false)
      (Variables|Default|SetLocationIndex 0))))