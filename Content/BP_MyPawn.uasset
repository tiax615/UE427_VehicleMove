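; BP_MyPawn is a self-driving vehicle pawn that follows a spline.
; BeginPlay caches the spline component from a referenced spline actor, and Tick holds a constant throttle.
; Each Tick also projects a look-ahead point in front of the pawn, finds the closest spline location and maps the yaw difference toward it into clamped steering input.
; The yaw difference is not normalized for angle wraparound.
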(event EventBeginPlay
  ;[1 1 1] Get Spline
  (Variables|Default|SetSplineBP (Actor|GetComponentbyClass (Variables|Default|GetSplineActorBP) "/Script/Engine.SplineComponent")))

(event EventTick
  (params (DeltaSeconds :type Float%20%28single-precision%29))
  (bind _returnvalue (Transformation|GetActorLocation))
  (Utilities|FlowControl|Sequence
    (:then_0
      (Class|WheeledVehicleMovementComponent|SetThrottleInput (Variables|Default|GetVehicleMovement) 0.6))
    (:then_1
      (Class|WheeledVehicleMovementComponent|SetSteeringInput (Variables|Default|GetVehicleMovement) (Math|Float|MapRangeClamped (- (.Yaw (Math|Rotator|BreakRotator (Math|Rotator|FindLookatRotation _returnvalue (Spline|FindLocationClosesttoWorldLocation (Variables|Default|GetSplineBP) (+ _returnvalue (* (Transformation|GetActorForwardVector) 2e+02)) "World")))) (.Yaw (Math|Rotator|BreakRotator (Transformation|GetActorRotation)))) -9e+01 9e+01 -1.0 1.0)))))

(fn ConstructionScript)